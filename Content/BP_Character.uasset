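; Player character Blueprint that drives movement, look, jump, crouch and a very high-speed sprint through Enhanced Input actions.
; FlipFlop toggles switch global slow motion, low gravity and spotlight visibility.
; The laser action line-traces a short range from the camera with debug drawing and spawns a BP_LaunchPack at the hit location, without checking that anything was hit.
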(event `EnhancedInput|/Game/Input/IA_move`
  (params (ActionValue :type "Vector2D Structure") (ElapsedSeconds :type "Float (double-precision)") (TriggeredSeconds :type "Float (double-precision)") (InputAction :type "InputAction Object Reference" :default "/Game/Input/IA_move.IA_move"))
  (:`Triggered`
    (`self.AddMovementInput` (`self.GetActorRightVector`) ActionValue_X)
    (`self.AddMovementInput` (`self.GetActorForwardVector`) ActionValue_Y)))

(event `EnhancedInput|/Game/Input/IA_sprint`
  (params (ActionValue :type Boolean) (ElapsedSeconds :type "Float (double-precision)") (TriggeredSeconds :type "Float (double-precision)") (InputAction :type "InputAction Object Reference" :default "/Game/Input/IA_sprint.IA_sprint"))
  (bind _charactermovement (`self.CharacterMovement`))
  (:`Triggered`
    (set `CharacterMovementComponent.MaxWalkSpeed` 120000.0 _charactermovement))
  (:`Completed`
    (set `CharacterMovementComponent.MaxWalkSpeed` 600.0 _charactermovement)))

(event `EnhancedInput|/Game/Input/IA_jump`
  (params (ActionValue :type Boolean) (ElapsedSeconds :type "Float (double-precision)") (TriggeredSeconds :type "Float (double-precision)") (InputAction :type "InputAction Object Reference" :default "/Game/Input/IA_jump.IA_jump"))
  (:`Triggered`
    (`self.Jump`))
  (:`Completed`
    (`self.StopJumping`)))

(event `EnhancedInput|/Game/Input/IA_look`
  (params (ActionValue :type "Vector2D Structure") (ElapsedSeconds :type "Float (double-precision)") (TriggeredSeconds :type "Float (double-precision)") (InputAction :type "InputAction Object Reference" :default "/Game/Input/IA_look.IA_look"))
  (:`Triggered`
    (`self.AddControllerYawInput` ActionValue_X)
    (`self.AddControllerPitchInput` ActionValue_Y)))

(event `EnhancedInput|/Game/Input/IA_Matrice`
  (params (ActionValue :type Boolean) (ElapsedSeconds :type "Float (double-precision)") (TriggeredSeconds :type "Float (double-precision)") (InputAction :type "InputAction Object Reference" :default "/Game/Input/IA_Matrice.IA_Matrice"))
  (:`Triggered`
    (`/Engine/EditorBlueprintResources/StandardMacros.FlipFlop`
      (:`A`
        (`GameplayStatics.SetGlobalTimeDilation` 0.3))
      (:`B`
        (`GameplayStatics.SetGlobalTimeDilation` 1.0)))))

(event `EnhancedInput|/Game/Input/IA_crouch`
  (params (ActionValue :type Boolean) (ElapsedSeconds :type "Float (double-precision)") (TriggeredSeconds :type "Float (double-precision)") (InputAction :type "InputAction Object Reference" :default "/Game/Input/IA_crouch.IA_crouch"))
  (:`Triggered`
    (`self.Crouch`))
  (:`Completed`
    (`self.UnCrouch`)))

(event `EnhancedInput|/Game/Input/IA_light`
  (params (ActionValue :type Boolean) (ElapsedSeconds :type "Float (double-precision)") (TriggeredSeconds :type "Float (double-precision)") (InputAction :type "InputAction Object Reference" :default "/Game/Input/IA_light.IA_light"))
  (:`Completed`
    (`/Engine/EditorBlueprintResources/StandardMacros.FlipFlop`
      (:`A`
        (`SceneComponent.SetHiddenInGame` (`self.SpotLight`) true false))
      (:`B`
        (`SceneComponent.SetHiddenInGame` (`self.SpotLight`) false false)))))

(event `EnhancedInput|/Game/Input/IA_gravity`
  (params (ActionValue :type Boolean) (ElapsedSeconds :type "Float (double-precision)") (TriggeredSeconds :type "Float (double-precision)") (InputAction :type "InputAction Object Reference" :default "/Game/Input/IA_gravity.IA_gravity"))
  (bind _charactermovement (`self.CharacterMovement`))
  (:`Triggered`
    (`/Engine/EditorBlueprintResources/StandardMacros.FlipFlop`
      (:`A`
        (set `CharacterMovementComponent.GravityScale` 0.1 _charactermovement))
      (:`B`
        (set `CharacterMovementComponent.GravityScale` 1.0 _charactermovement)))))

(event `EnhancedInput|/Game/Input/IA_laser`
  (params (ActionValue :type Boolean) (ElapsedSeconds :type "Float (double-precision)") (TriggeredSeconds :type "Float (double-precision)") (InputAction :type "InputAction Object Reference" :default "/Game/Input/IA_laser.IA_laser"))
  (bind _camera (`self.Camera`))
  (bind _returnvalue (`SceneComponent.K2_GetComponentLocation` _camera))
  (:`Completed`
    (bind _outhit (`KismetSystemLibrary.LineTraceSingle` :`Start` _returnvalue :`End` (+ _returnvalue (* (`SceneComponent.GetForwardVector` _camera) 1000.0)) :`TraceChannel` "TraceTypeQuery1" :`DrawDebugType` "ForDuration"))
    (`|SpawnActorFromClass` "/Game/BP_LaunchPack.BP_LaunchPack_C" (`KismetMathLibrary.MakeTransform` (`.Location` (`GameplayStatics.BreakHitResult` _outhit))) "Undefined" "MultiplyWithRoot" null (0.0 0.0 0.0) null)))

(fn `UserConstructionScript`)